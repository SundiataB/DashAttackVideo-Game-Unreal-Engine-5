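; Meteor attack spawner that grows its Portal mesh on BeginPlay, then starts a repeating meteorite strike, also triggerable through BeginAttack2.
; Each strike picks a random navigable point around the Sphere's relative location, spawning a scaled-up BP_MeteoriteDamage overhead and a tall BP_AntiGravityZone there.
; SpawnPortal re-calls itself through a resettable DoOnce until the counter reaches 100.
; The clamped RandomFloat delay always yields the two-second minimum.
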(event `SpawnPortal`
  (`/Engine/EditorBlueprintResources/StandardMacros.DoOnce` false :!label _label
    (:`Completed`
      (bind _randomlocation (`NavigationSystemV1.K2_GetRandomLocationInNavigableRadius` (`SceneComponent.RelativeLocation` (`self.Sphere`)) 5000.0 null null))
      (bind _returnvalue (`|SpawnActorFromClass` "/Game/Blueprints/BP_MeteoriteDamage.BP_MeteoriteDamage_C" (`KismetMathLibrary.MakeTransform` (`KismetMathLibrary.MakeVector` (.x _randomlocation) (.y _randomlocation) 1500.0)) "Undefined" "MultiplyWithRoot" null null))
      (bind _returnvalue_2 (`|SpawnActorFromClass` "/Game/Blueprints/BP_AntiGravityZone.BP_AntiGravityZone_C" (`KismetMathLibrary.MakeTransform` (`KismetMathLibrary.MakeVector` (.x _randomlocation) (.y _randomlocation)) (struct) (10.0 10.0 50.0)) "Undefined" "MultiplyWithRoot" null null))
      (`/Game/Blueprints/BP_MeteoriteDamage.scale up` _returnvalue)
      (bind _result (`/Engine/EditorBlueprintResources/StandardMacros.IncrementInt` (`self.counter`))
        (:`  `
          (set `self.counter` _result)
          (`self.ResetSpawner`)
          (if (not (> (`self.counter`) 99))
            ;[0.02079 1 0 0.5] Meg -Delay before next portal spawned
            (`KismetSystemLibrary.Delay` (`KismetMathLibrary.FClamp` (`KismetMathLibrary.RandomFloat`) 2.0 7.0))
            (`self.SpawnPortal`)))))))

(event `BeginAttack2`
  (`KismetSystemLibrary.Delay` 0.0 :!label _label_2)
  (goto _label))

(event `ResetSpawner`
  (goto _label :!via `Reset`))

(event `self.ReceiveBeginPlay`
  (bind __portal (`self. Portal`))
  (bind (_direction _newtrack_0) (`Timeline|Timeline`)
    (:`Update`
      (`SceneComponent.K2_SetRelativeTransform` __portal (`KismetMathLibrary.MakeTransform` (`SceneComponent.RelativeLocation` __portal) (struct) (* _newtrack_0 (5.0 5.0 1.0))) false false))
    (:`Finished`
      (goto _label_2))))

(fn `UserConstructionScript`)