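; Conveyor belt actor that fakes a moving surface by repeatedly nudging and resetting its Movement component.
; Each Tick resets Movement to its origin, then a FlipFlop alternates starting a MoveComponentTo along X scaled by Speed with resetting and stopping it.
; CollisionObj's physical material switches between frictionless and rubber on those alternate ticks.
; The construction script locks actor scale to one and sizes Movement from Size as a thin slab.
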(event `self.ReceiveTick`
  (params (DeltaSeconds :type "Float (single-precision)"))
  (`SceneComponent.K2_SetRelativeLocation` (`self.Movement`) (0.0 0.0 0.0) false false)
  (`/Engine/EditorBlueprintResources/StandardMacros.FlipFlop`
    (:`A`
      (`PrimitiveComponent.SetPhysMaterialOverride` (`self.CollisionObj`) "/Game/Meshes/ConveyorBelt/CB1/PM_NoFriction.PM_NoFriction")
      (`KismetSystemLibrary.MoveComponentTo` (`self.Movement`) (`KismetMathLibrary.MakeVector` (`self.Speed`)) (struct) false false 1.0 :!label _label))
    (:`B`
      (`PrimitiveComponent.SetPhysMaterialOverride` (`self.CollisionObj`) "/Engine/EngineMaterials/PhysMat_Rubber.PhysMat_Rubber")
      (`SceneComponent.K2_SetRelativeLocation` (`self.Movement`) (0.0 0.0 0.0) false false)
      (`|ExecutionSequence`
        (:`then_0`
          (goto _label :!via `Return`))
        (:`then_1`
          (goto _label :!via `Stop`))))))

(fn `UserConstructionScript`
  (bind (_size_x _size_y) (`KismetMathLibrary.BreakVector2D` (`self.Size`)))
  (`self.SetActorScale3D` (1.0 1.0 1.0))
  (`SceneComponent.SetRelativeScale3D` (`self.Movement`) (`KismetMathLibrary.MakeVector` _size_x _size_y 0.03)))