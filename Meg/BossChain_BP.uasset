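; Boss chain actor built on a Cable component, whose end can break loose to become a burning hazard.
; DettachEnd waits briefly, frees the cable end, then attaches sparks, a temporary torch fire effect and a hidden, spawned purple-plane damage actor to the CableEnd socket.
; BeginPlay caches the third-person player, while PlaySmoke is empty and the player-tag check is unconnected.
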(event `self.ReceiveBeginPlay`
  (bind _asbp_third_person_character (cast `/Game/ThirdPerson/Blueprints/BP_ThirdPersonCharacter` (`GameplayStatics.GetPlayerPawn` 0)))
  (set `self.PlayerRef` _asbp_third_person_character))

(event `DettachEnd`
  (bind _cable (`self.Cable`))
  (`KismetSystemLibrary.Delay` 0.2)
  (set `CableComponent.bAttachEnd` false _cable)
  (`GameplayStatics.SpawnEmitterAttached` "/Game/StarterContent/Particles/P_MySparks.P_MySparks" _cable "CableEnd" (0.0 0.0 10.0) (struct) (10.0 10.0 10.0))
  (bind _returnvalue (`|SpawnActorFromClass` "/Game/Meshes/PurplePlaneDamage_BP.PurplePlaneDamage_BP_C" (`KismetMathLibrary.MakeTransform` (0.0 0.0 0.0) (struct :`Yaw` 90.0)) "Undefined" "MultiplyWithRoot" null null))
  (`self.SetActorHiddenInGame` _returnvalue true)
  (`self.K2_AttachToComponent` _returnvalue (`self.Cable`) "CableEnd" "KeepRelative" "KeepRelative" "KeepRelative" true)
  (set `self.PlayerCollided` false)
  (bind _returnvalue_2 (`GameplayStatics.SpawnEmitterAttached` "/Game/Effects/Particles/Fire/P_TorchFire.P_TorchFire" _cable "CableEnd" (0.0 0.0 0.0) (struct) (20.0 20.0 20.0)))
  (`KismetSystemLibrary.Delay` 10.0)
  (`ActorComponent.Deactivate` _returnvalue_2))

(event `PlaySmoke`)

(fn `UserConstructionScript`)