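; WorkerBot1_BP is a worker bot actor that moves along a referenced spline, starting at BeginPlay.
; A timeline with its play rate scaled by the inverse of TimeToComplete drives a 0-to-1 blend over the spline's length.
; Each update places the actor at that world-space distance along the spline without sweeping or changing rotation.
; The construction script applies a configurable static mesh.
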(event `self.ReceiveBeginPlay`
  (`self.HoverObject`))

(event `HoverObject`
  (bind _spline (`/Game/Meshes/ConveyorBelt/CB2/SplinePath_BP.Spline` (`self.SplineToFollow`)))
  (`TimelineComponent.SetPlayRate` (`self.T_Hover`) (/ 1.0 (`self.TimeToComplete`)))
  (bind (_direction _hovermove) (`Timeline|T_Hover`)
    (:`Update`
      (`self.K2_SetActorLocation` (`SplineComponent.GetLocationAtDistanceAlongSpline` _spline (`KismetMathLibrary.Lerp` 0.0 (`SplineComponent.GetSplineLength` _spline) _hovermove) "World")))))

(fn `UserConstructionScript`
  (`StaticMeshComponent.SetStaticMesh` (`self.StaticMesh`) (`self.ObjectStaticMesh`)))