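; SplineObject_BP is an actor that carries a configurable static mesh along another actor's spline, likely as an item on a conveyor belt.
; The construction script applies the chosen mesh, and BeginPlay starts the move automatically.
; A timeline, with play rate scaled by the inverse of TimeToComplete, maps its track to distance along the spline.
; Each update sets the actor's world location and rotation from that point.
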(event `self.ReceiveBeginPlay`
  (`self.Move Object`))

(event `Move Object`
  (bind _spline (`/Game/Meshes/ConveyorBelt/CB2/SplinePath_BP.Spline` (`self.SplineToFollow`)))
  (`TimelineComponent.SetPlayRate` (`self.T_Move`) (/ 1.0 (`self.TimeToComplete`)))
  (bind (_direction _movetrack) (`Timeline|T_Move`)
    (:`Update`
      (bind _returnvalue (`KismetMathLibrary.Lerp` 0.0 (`SplineComponent.GetSplineLength` _spline) _movetrack))
      (`self.K2_SetActorLocationAndRotation` (`SplineComponent.GetLocationAtDistanceAlongSpline` _spline _returnvalue "World") (`SplineComponent.GetRotationAtDistanceAlongSpline` _spline _returnvalue "World")))))

(fn `UserConstructionScript`
  (`StaticMeshComponent.SetStaticMesh` (`self.StaticMesh`) (`self.ObjectStaticMesh`)))