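; Skull projectile Blueprint whose own logic adds flight and impact audio on top of its parent class.
; On BeginPlay it attaches a missile movement sound to the collision box and keeps the audio component.
; When the box registers a hit, that same component's sound is swapped to an explosion instead of spawning a new one.
; Overlap and construction only call the parent, and Tick is disabled.
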(event `self.ReceiveBeginPlay`
  (`parent.ReceiveBeginPlay`)
  ;[0.0239 1 0 0.5] Meg-create sound of moving missle, attached to collision box with attenuation enabled
  (bind _returnvalue (`GameplayStatics.SpawnSoundAttached` "/Game/Audio/Dash_Attack_-_MissleMovement.Dash_Attack_-_MissleMovement" (`self.BoxCollision`) "None" (0.0 0.0 0.0) (struct) "KeepRelativeOffset" false 1.0 1.0 0.0 null null))
  (set `self.MissleSound` _returnvalue))

(event `self.ReceiveActorBeginOverlap`
  (params (OtherActor :type "Actor Object Reference"))
  (`parent.ReceiveActorBeginOverlap` OtherActor))

(event `self.BoxCollision.OnComponentHit`
  (params (HitComponent :type "PrimitiveComponent Object Reference") (OtherActor :type "Actor Object Reference") (OtherComp :type "PrimitiveComponent Object Reference") (NormalImpulse :type "Vector Structure") (Hit :type "HitResult Structure (by ref)"))
  (bind _misslesound (`self.MissleSound`))
  ;[0 1 0.1674 0.5] Meg-Change sound to "impact" once missle collides
  (`/Engine/EditorBlueprintResources/StandardMacros.IsValid` _misslesound
    (:`Is Valid`
      (`AudioComponent.SetSound` _misslesound "/Game/StarterContent/Audio/Explosion01.Explosion01"))))

(fn `UserConstructionScript`
  (`parent.UserConstructionScript`))