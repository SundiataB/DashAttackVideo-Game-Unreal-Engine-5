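; BP_Enemy_Base is an enemy base Blueprint that exposes health, healing and damage functions backed by a DamageSystemBPC component.
; GetCurrentHealth and GetMaxHealth read the component's values, while Heal and TakeDamage forward their arguments to it and return its results.
; BeginPlay and the construction script are empty, so the Blueprint's graphs hold no behavior beyond this delegation.
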(event `self.ReceiveBeginPlay`)

(fn `GetCurrentHealth`
  (returns (Health :type "Float (double-precision)"))
  (return (`/Game/ThirdPerson/Systems/DamageSystem/DamageSystem_BPC.Health` (`self.DamageSystem_BPC`))))

(fn `GetMaxHealth`
  (returns (MaxHealth :type "Float (double-precision)"))
  (return (`/Game/ThirdPerson/Systems/DamageSystem/DamageSystem_BPC.MaxHealth` (`self.DamageSystem_BPC`))))

(fn `Heal`
  (params (Amount :type "Float (double-precision)"))
  (returns (NewHealth :type "Float (double-precision)"))
  (bind _newhealth (`/Game/ThirdPerson/Systems/DamageSystem/DamageSystem_BPC.Heal` (`self.DamageSystem_BPC`) Amount))
  (return _newhealth))

(fn `TakeDamage`
  (params (DamageInfo :type "/Game/ThirdPerson/Systems/DamageSystem/DamageInfo_S Structure"))
  (returns (WasDamaged :type Boolean))
  (bind _wasdamaged (`/Game/ThirdPerson/Systems/DamageSystem/DamageSystem_BPC.TakeDamage` (`self.DamageSystem_BPC`) DamageInfo))
  (return _wasdamaged))

(fn `UserConstructionScript`)