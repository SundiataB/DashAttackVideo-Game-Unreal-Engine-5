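; BP_Explosive_Base is an explosive actor that detonates when a Projectile- or Player-tagged actor overlaps its sphere.
; After a short delay it spawns explosion effects and sound, sends damage to the cached player, then destroys itself.
; The player is cached on BeginPlay regardless of distance and cleared permanently on leaving the sphere, so damage skips only a player who entered and left.
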(event `self.ReceiveBeginPlay`
  (bind _asbp_third_person_character (cast `/Game/ThirdPerson/Blueprints/BP_ThirdPersonCharacter` (`GameplayStatics.GetPlayerCharacter` 0)))
  (set `self.PlayerREF` _asbp_third_person_character)
  (set `self.MeshToSpawn` null))

(event `self.Sphere.OnComponentBeginOverlap`
  (params (OverlappedComponent :type "PrimitiveComponent Object Reference") (OtherActor :type "Actor Object Reference") (OtherComp :type "PrimitiveComponent Object Reference") (OtherBodyIndex :type Integer) (bFromSweep :type Boolean) (SweepResult :type "HitResult Structure (by ref)"))
  (bind _returnvalue (`SceneComponent.K2_GetComponentLocation` (`self.Sphere`)))
  (if (or (`self.ActorHasTag` OtherActor "Projectile") (`self.ActorHasTag` OtherActor "Player"))
    (`KismetSystemLibrary.Delay` 0.5)
    (`GameplayStatics.SpawnEmitterAtLocation` "/Game/StarterContent/Particles/P_Explosion.P_Explosion" _returnvalue (struct) (3.0 3.0 3.0))
    (`GameplayStatics.PlaySoundAtLocation` "/Game/StarterContent/Audio/Explosion01.Explosion01" _returnvalue (struct) 1.0 1.0 0.0 null null null null)
    (if (`KismetSystemLibrary.IsValid` (`self.PlayerREF`))
      (message `/Game/ThirdPerson/Systems/DamageSystem/Damageable_BPI.TakeDamage` (`self.PlayerREF`) (make `/Game/ThirdPerson/Systems/DamageSystem/DamageInfo_S` 25.0 "NewEnumerator3" "NewEnumerator1")))
    (`self.K2_DestroyActor`)))

(event `self.Sphere.OnComponentEndOverlap`
  (params (OverlappedComponent :type "PrimitiveComponent Object Reference") (OtherActor :type "Actor Object Reference") (OtherComp :type "PrimitiveComponent Object Reference") (OtherBodyIndex :type Integer))
  (if (`self.ActorHasTag` OtherActor "Player")
    (set `self.PlayerREF` null)))

(fn `UserConstructionScript`)