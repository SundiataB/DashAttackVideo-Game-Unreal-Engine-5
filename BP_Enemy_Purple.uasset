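; Purple robot enemy that chases the player on sight, alternating a delayed right-side laser with a charged left-side homing missile or skull.
; Pawn sensing drives movement and firing, and projectile impact events deal damage, with camera shake on left-side hits.
; Health runs through DamageSystemBPC, and death spawns a GC_BP_Robot_Mech and updates the WaveDirector count.
; An overlap sphere toggles its HUD widget and purple overlay near the player.
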(event `CameraShake`
  ;[0.5 0 1 1 40] Camera Shake Event on Missile Hit
  (bind _asplayer_controller (cast `PlayerController` (`self.GetController` (`self.PlayerREF`))))
  (bind _output_get (set `self.PlayerControllerREF` _asplayer_controller))
  (`PlayerController.ClientStartCameraShake` :`self` _output_get :`Shake` "/Game/Enemy/Projectiles/BP_CameraShake.BP_CameraShake_C" :`PlaySpace` "World"))

(event `self.Widget&OverlaySphere.OnComponentBeginOverlap`
  (params (OverlappedComponent :type "PrimitiveComponent Object Reference") (OtherActor :type "Actor Object Reference") (OtherComp :type "PrimitiveComponent Object Reference") (OtherBodyIndex :type Integer) (bFromSweep :type Boolean) (SweepResult :type "HitResult Structure (by ref)"))
  ;[0.5 0 1 1 40] Widget view distance
  (if (`self.ActorHasTag` OtherActor "Player")
    (`SceneComponent.SetVisibility` (`self.Widget`) true false)
    (`MeshComponent.SetOverlayMaterial` (`self.Mesh`) "/Game/ThirdPerson/Systems/Tutorial/TutorialText/VFX/MaterialsOverlay/MI_OverlayPurple.MI_OverlayPurple")))

(event `PurpleDeath`
  ;[0.5 0 1 1 40] Death
  (`|SpawnActorFromClass` "/Game/Enemy/Robots/RobotMech_SM_GC/GC_BP_Robot_Mech.GC_BP_Robot_Mech_C" (`KismetMathLibrary.Conv_VectorToTransform` (`SceneComponent.K2_GetComponentLocation` (`self.Mesh`))) "Undefined" "MultiplyWithRoot" null null)
  (`self.K2_DestroyActor`)
  (bind _aswave_director (cast `/Game/LevelPrototyping/Marceyas/WaveDirector` (`self.WaveDirector`))
    (:`then`
      (`/Game/LevelPrototyping/Marceyas/WaveDirector.CountCall` _aswave_director)
      (`/Game/LevelPrototyping/Marceyas/WaveDirector.CountCheck` _aswave_director))
    (:`CastFailed`
      (`KismetSystemLibrary.PrintString` "Fail"))))

(event `self.ReceiveBeginPlay`
  (bind _charactermovement (`self.CharacterMovement`))
  ;[0.5 0 1 1 40] BeginPlay
  (bind _asbp_third_person_character (cast `/Game/ThirdPerson/Blueprints/BP_ThirdPersonCharacter` (`GameplayStatics.GetPlayerCharacter` 0)))
  (set `self.PlayerREF` _asbp_third_person_character)
  (bind _returnvalue (`|CreateWidget` "/Game/ThirdPerson/Widgets/purpleHUD_W.purpleHUD_W_C" null self))
  (`WidgetComponent.SetWidget` (`self.Widget`) _returnvalue)
  (`SceneComponent.SetVisibility` (`self.Widget`) false false)
  (set `CharacterMovementComponent.MaxWalkSpeed` (`self.MaxWalkSpeed`) _charactermovement)
  (set `CharacterMovementComponent.GroundFriction` (`self.GroundFriction`) _charactermovement)
  (bind _returnvalue_2 (`GameplayStatics.GetActorOfClass` "/Game/LevelPrototyping/Marceyas/WaveDirector.WaveDirector_C"))
  (set `self.WaveDirector` _returnvalue_2))

(event `self.Widget&OverlaySphere.OnComponentEndOverlap`
  (params (OverlappedComponent :type "PrimitiveComponent Object Reference") (OtherActor :type "Actor Object Reference") (OtherComp :type "PrimitiveComponent Object Reference") (OtherBodyIndex :type Integer))
  ;[0.5 0 1 1 40] Widget view distance
  (if (`self.ActorHasTag` OtherActor "Player")
    (`SceneComponent.SetVisibility` (`self.Widget`) false false)
    (`MeshComponent.SetOverlayMaterial` (`self.Mesh`) null)))

(event `self.PawnSensing.OnSeePawn`
  (params (Pawn :type "Pawn Object Reference"))
  (bind _p_misslecharge (`self.P_MissleCharge`))
  (bind (_returnvalue_roll _returnvalue_pitch _returnvalue_yaw) (`KismetMathLibrary.BreakRotator` (`KismetMathLibrary.FindLookAtRotation` (`SceneComponent.K2_GetComponentLocation` (`self.Mesh`)) (`PlayerController.GetFocalLocation` (`GameplayStatics.GetPlayerController` 0)))))
  ;[0.5 0 1 1 50] Acceptance Radius + pawnsensing sight radius   -----  pawnsensing interval dictates initial rates of firing
  (if (`self.ActorHasTag` Pawn "Player")
    (`SceneComponent.K2_SetWorldRotation` (`self.Mesh`) (`KismetMathLibrary.MakeRotator` 0.0 0.0 (+ _returnvalue_yaw -90.0)) false true)
    (`|AIMoveTo` (`self.PawnSensing`) self (0.0 0.0 0.0) Pawn (`self.AcceptanceRadius`)
      (:`OnSuccess`
        (bind _returnvalue (`GameplayStatics.GetActorOfClass` "/Game/ThirdPerson/Blueprints/BP_ThirdPersonCharacter.BP_ThirdPersonCharacter_C"))
        (set `self.Target` _returnvalue)
        (`/Engine/EditorBlueprintResources/StandardMacros.FlipFlop`
          (:`A`
            (`KismetSystemLibrary.Delay` 1.0)
            (`self.ShootR`))
          (:`B`
            ;;[1 0.3219 0 0.5] Meg-Charge up Missle attack "5 seconds to charge. Will not spawn another until completed"
            (if (not (`ActorComponent.IsActive` _p_misslecharge))
              (`KismetSystemLibrary.PrintString` (`KismetSystemLibrary.GetDisplayName` _p_misslecharge))
              (`AudioComponent.Play` (`self.Dash_Attack_-_MissleCharge1__1_`) 0.0)
              (`ActorComponent.Activate` _p_misslecharge false)
              (`KismetSystemLibrary.Delay` 5.0)
              (`self.ShootL`)
              (`ActorComponent.Deactivate` (`self.P_MissleCharge`)))))))))

(event `ShootL`
  (bind (_returnvalue_location _returnvalue_rotation _returnvalue_scale) (`KismetMathLibrary.BreakTransform` (`SceneComponent.K2_GetComponentToWorld` (`self.TempEjectorScene_L`))))
  ;[0.5 0 1 1 50] Acceptance Radius + pawnsensing sight radius   -----  pawnsensing interval dictates initial rates of firing
  (if (not (`/Game/ThirdPerson/Systems/DamageSystem/DamageSystem_BPC.bIsDead` (`self.DamageSystem_BPC`)))
    (`GameplayStatics.SpawnEmitterAtLocation` "/Game/StarterContent/Particles/P_Explosion.P_Explosion" _returnvalue_location _returnvalue_rotation _returnvalue_scale)
    (bind _returnvalue (`|SpawnActorFromClass` (select `int` (`KismetMathLibrary.RandomInteger` 2) :`0` "/Game/Enemy/Projectiles/Projectile_Missile_BP.Projectile_Missile_BP_C" :`1` "/Game/Enemy/Projectiles/Projectile_Skull_BP.Projectile_Skull_BP_C" :!type "/Game/Enemy/Projectiles/Projectile_Base_BP Class Reference") (`SceneComponent.K2_GetComponentToWorld` (`self.TempEjectorScene_L`)) "Undefined" "MultiplyWithRoot" self 1750.0 0.0 (`self.Target`) true null))
    (add `/Game/Enemy/Projectiles/Projectile_Base_BP.OnProjectileImpact` _returnvalue (`|CreateDelegate` :!event `MissileL`))
    (`PrimitiveComponent.IgnoreActorWhenMoving` (`self.CapsuleComponent`) _returnvalue true)))

(event `ShootR`
  (bind (_returnvalue_location _returnvalue_rotation _returnvalue_scale) (`KismetMathLibrary.BreakTransform` (`SceneComponent.K2_GetComponentToWorld` (`self.TempEjectorScene_R`))))
  ;[0.5 0 1 1 50] Acceptance Radius + pawnsensing sight radius   -----  pawnsensing interval dictates initial rates of firing
  (if (not (`/Game/ThirdPerson/Systems/DamageSystem/DamageSystem_BPC.bIsDead` (`self.DamageSystem_BPC`)))
    (`GameplayStatics.SpawnEmitterAtLocation` "/Game/StarterContent/Particles/P_Explosion.P_Explosion" _returnvalue_location _returnvalue_rotation _returnvalue_scale)
    (bind _returnvalue (`|SpawnActorFromClass` (select `int` (`KismetMathLibrary.RandomInteger` 1) :`0` "/Game/Enemy/Projectiles/Projectile_Laser_BP.Projectile_Laser_BP_C" :`1` null :!type "/Game/Enemy/Projectiles/Projectile_Base_BP Class Reference") (`SceneComponent.K2_GetComponentToWorld` (`self.TempEjectorScene_R`)) "Undefined" "MultiplyWithRoot" self 7500.0 0.0 (`self.Target`) false null))
    (add `/Game/Enemy/Projectiles/Projectile_Base_BP.OnProjectileImpact` _returnvalue (`|CreateDelegate` :!event `LaserR`))
    (`PrimitiveComponent.IgnoreActorWhenMoving` (`self.CapsuleComponent`) _returnvalue true)))

(event `PurpleBlocked`
  (params (CanBeParried :type Boolean)))

(event `LaserR`
  (params (`Other Actor` :type "Actor Object Reference") (Hit :type "HitResult Structure"))
  (bind (_bblockinghit _binitialoverlap _time _distance _location _impactpoint _normal _impactnormal _physmat _hitactor) (`GameplayStatics.BreakHitResult` Hit))
  ;[0.5 0 1 1 50] Acceptance Radius + pawnsensing sight radius   -----  pawnsensing interval dictates initial rates of firing
  (if (`self.ActorHasTag` _hitactor "Player")
    (if (not (`/Game/ThirdPerson/Blueprints/BP_ThirdPersonCharacter.bIsDamageCauserActive` (`self.PlayerREF`)))
      (bind _wasdamaged (message `/Game/ThirdPerson/Systems/DamageSystem/Damageable_BPI.TakeDamage` _hitactor (make `/Game/ThirdPerson/Systems/DamageSystem/DamageInfo_S` 10.0 "NewEnumerator2" "NewEnumerator1")))
      (if _wasdamaged
        (`GameplayStatics.SpawnEmitterAtLocation` "/Game/StarterContent/Particles/P_Explosion.P_Explosion")))))

(event `MissileL`
  (params (`Other Actor` :type "Actor Object Reference") (Hit :type "HitResult Structure"))
  (bind (_bblockinghit _binitialoverlap _time _distance _location _impactpoint _normal _impactnormal _physmat _hitactor) (`GameplayStatics.BreakHitResult` Hit))
  ;[0.5 0 1 1 50] Acceptance Radius + pawnsensing sight radius   -----  pawnsensing interval dictates initial rates of firing
  (if (`self.ActorHasTag` _hitactor "Player")
    (if (not (`/Game/ThirdPerson/Blueprints/BP_ThirdPersonCharacter.bIsDamageCauserActive` (`self.PlayerREF`)))
      (bind _wasdamaged (message `/Game/ThirdPerson/Systems/DamageSystem/Damageable_BPI.TakeDamage` _hitactor (make `/Game/ThirdPerson/Systems/DamageSystem/DamageInfo_S` 10.0 "NewEnumerator2" "NewEnumerator1")))
      (if _wasdamaged
        (`GameplayStatics.SpawnEmitterAtLocation` "/Game/StarterContent/Particles/P_Explosion.P_Explosion")
        (`self.CameraShake`)))))

(event `PurpleDamageResponse`
  (params (DamageResponse :type "/Game/ThirdPerson/Systems/DamageSystem/DamageResponse_E Enum" :default "NewEnumerator0")))

(fn `GetCurrentHealth`
  (returns (Health :type "Float (double-precision)"))
  (return (`/Game/ThirdPerson/Systems/DamageSystem/DamageSystem_BPC.Health` (`self.DamageSystem_BPC`))))

(fn `GetMaxHealth`
  (returns (MaxHealth :type "Float (double-precision)"))
  (return (`/Game/ThirdPerson/Systems/DamageSystem/DamageSystem_BPC.MaxHealth` (`self.DamageSystem_BPC`))))

(fn `Heal`
  (params (Amount :type "Float (double-precision)"))
  (returns (NewHealth :type "Float (double-precision)"))
  (bind _newhealth (`/Game/ThirdPerson/Systems/DamageSystem/DamageSystem_BPC.Heal` (`self.DamageSystem_BPC`) Amount))
  (return _newhealth))

(fn `TakeDamage`
  (params (DamageInfo :type "/Game/ThirdPerson/Systems/DamageSystem/DamageInfo_S Structure"))
  (returns (WasDamaged :type Boolean))
  (bind _wasdamaged (`/Game/ThirdPerson/Systems/DamageSystem/DamageSystem_BPC.TakeDamage` (`self.DamageSystem_BPC`) DamageInfo))
  (return _wasdamaged))

(fn `UserConstructionScript`
  (bind _damagesystem_bpc (`self.DamageSystem_BPC`))
  (add `/Game/ThirdPerson/Systems/DamageSystem/DamageSystem_BPC.OnDeath` _damagesystem_bpc (`|CreateDelegate` :!event `PurpleDeath`))
  (add `/Game/ThirdPerson/Systems/DamageSystem/DamageSystem_BPC.OnBlocked` _damagesystem_bpc (`|CreateDelegate` :!event `PurpleBlocked`))
  (add `/Game/ThirdPerson/Systems/DamageSystem/DamageSystem_BPC.OnDamageResponse` _damagesystem_bpc (`|CreateDelegate` :!event `PurpleDamageResponse`)))