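; BP_AntiGravityZone is a temporary zone actor that switches off gravity for actors inside it and destroys itself five seconds after BeginPlay.
; Begin and end overlap on its Zone component send ToggleGravityMessage off and on to actors implementing BPI_AntiGravity, leaving each receiver to handle the change.
; A global toggle over all implementing actors remains as disconnected nodes, and its ToggleAllGravity event is empty.
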(event `self.ReceiveBeginPlay`
  (`KismetSystemLibrary.Delay` 5.0)
  (`self.K2_DestroyActor`))

(event `self.Zone.OnComponentBeginOverlap`
  (params (OverlappedComponent :type "PrimitiveComponent Object Reference") (OtherActor :type "Actor Object Reference") (OtherComp :type "PrimitiveComponent Object Reference") (OtherBodyIndex :type Integer) (bFromSweep :type Boolean) (SweepResult :type "HitResult Structure (by ref)"))
  (if (`KismetSystemLibrary.DoesImplementInterface` OtherActor "/Game/Blueprints/BPI_AntiGravity.BPI_AntiGravity_C")
    (message `/Game/Blueprints/BPI_AntiGravity.ToggleGravity` OtherActor false)))

(event `self.Zone.OnComponentEndOverlap`
  (params (OverlappedComponent :type "PrimitiveComponent Object Reference") (OtherActor :type "Actor Object Reference") (OtherComp :type "PrimitiveComponent Object Reference") (OtherBodyIndex :type Integer))
  (if (`KismetSystemLibrary.DoesImplementInterface` OtherActor "/Game/Blueprints/BPI_AntiGravity.BPI_AntiGravity_C")
    (message `/Game/Blueprints/BPI_AntiGravity.ToggleGravity` OtherActor true)))

(event `ToggleAllGravity`
  (params (hasGravity :type Boolean)))

(fn `UserConstructionScript`)