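; Tutorial trigger volume that unlocks the player's jump and dash and shows a tutorial text actor while the player stands inside it.
; On player overlap, after a short delay, it enables both abilities on the third-person character and spawns TutorialText_PPU_BP at a hardcoded world location.
; When the player leaves, it re-enables both abilities, then destroys the trigger box and the text actor, so the step runs once.
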(event `self.ReceiveBeginPlay`
  (bind _asbp_third_person_character (cast `/Game/ThirdPerson/Blueprints/BP_ThirdPersonCharacter` (`GameplayStatics.GetPlayerCharacter` 0)))
  (set `self.PlayerREF` _asbp_third_person_character))

(event `self.Trigger5Box.OnComponentBeginOverlap`
  (params (OverlappedComponent :type "PrimitiveComponent Object Reference") (OtherActor :type "Actor Object Reference") (OtherComp :type "PrimitiveComponent Object Reference") (OtherBodyIndex :type Integer) (bFromSweep :type Boolean) (SweepResult :type "HitResult Structure (by ref)"))
  (if (`self.ActorHasTag` OtherActor "Player")
    (`KismetSystemLibrary.Delay` 0.2)
    (bind _asbp_third_person_character (cast `/Game/ThirdPerson/Blueprints/BP_ThirdPersonCharacter` (`GameplayStatics.GetPlayerCharacter` 0)))
    (set `/Game/ThirdPerson/Blueprints/BP_ThirdPersonCharacter.bCanJump` true _asbp_third_person_character)
    (set `/Game/ThirdPerson/Blueprints/BP_ThirdPersonCharacter.bCanDash` true _asbp_third_person_character)
    (bind _returnvalue (`|SpawnActorFromClass` "/Game/ThirdPerson/Systems/Tutorial/TutorialText/Trigs_Text/TutorialText_PPU_BP.TutorialText_PPU_BP_C" (`KismetMathLibrary.MakeTransform` (-23500.0 0.0 1000.0)) "Undefined" "MultiplyWithRoot" null null))
    (set `self.PPUText_REF` _returnvalue)))

(event `self.Trigger5Box.OnComponentEndOverlap`
  (params (OverlappedComponent :type "PrimitiveComponent Object Reference") (OtherActor :type "Actor Object Reference") (OtherComp :type "PrimitiveComponent Object Reference") (OtherBodyIndex :type Integer))
  (bind _playerref (`self.PlayerREF`))
  (if (`self.ActorHasTag` OtherActor "Player")
    (`KismetSystemLibrary.Delay` 0.2)
    (set `/Game/ThirdPerson/Blueprints/BP_ThirdPersonCharacter.bCanJump` true _playerref)
    (set `/Game/ThirdPerson/Blueprints/BP_ThirdPersonCharacter.bCanDash` true _playerref)
    (`ActorComponent.K2_DestroyComponent` (`self.Trigger5Box`))
    (`self.K2_DestroyActor` (`self.PPUText_REF`))))

(fn `UserConstructionScript`)