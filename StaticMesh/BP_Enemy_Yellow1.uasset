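; Yellow melee enemy Blueprint that chases the player on sight and attacks with a weapon.
; PawnSensing reveals the health-interface widget and starts AIMoveTo, which triggers a random montage whose notify sphere-traces between weapon sockets to deal damage.
; DamageSystemBPC backs the damage, heal and health functions and drives death, which ragdolls the mesh, hides effects and destroys the actor.
; Blocked and damage-response handlers are bound but empty.
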(event `self.ReceiveBeginPlay`
  ;[1 0.7149 0 1 50] Begin Play
  (bind _asbp_third_person_character (cast `/Game/ThirdPerson/Blueprints/BP_ThirdPersonCharacter` (`GameplayStatics.GetPlayerCharacter` 0)))
  (set `self.PlayerREF` _asbp_third_person_character)
  (bind _returnvalue (`|CreateWidget` "/Game/ThirdPerson/Widgets/yellowHUD_W.yellowHUD_W_C" null self))
  (`WidgetComponent.SetWidget` (`self.Widget`) _returnvalue)
  (`SceneComponent.SetVisibility` (`self.Widget`) false false))

(event `YellowDeath`
  (bind _mesh (`self.Mesh`))
  ;[1 0.7149 0 1 50] Death
  (`PrimitiveComponent.SetSimulatePhysics` _mesh true)
  (`PrimitiveComponent.SetCollisionEnabled` _mesh "QueryAndPhysics")
  (`ActorComponent.K2_DestroyComponent` (`self.CapsuleComponent`))
  (`SceneComponent.SetVisibility` (`self.Widget`) false false)
  (`SceneComponent.SetVisibility` (`self.SteamLegL`) false false)
  (`SceneComponent.SetVisibility` (`self.SteamLegR`) false false)
  (`SceneComponent.SetVisibility` (`self.SteamBod`) false false)
  (`KismetSystemLibrary.Delay` 1.0)
  (`self.K2_DestroyActor`))

(event `self.PawnSensing.OnSeePawn`
  (params (Pawn :type "Pawn Object Reference"))
  ;[1 0.7149 0 1 50] Pawn Sense + Attack
  (if (`self.ActorHasTag` Pawn "Player")
    (`SceneComponent.SetVisibility` (`self.Widget`) true false)
    (`|AIMoveTo` (`self.PawnSensing`) self (0.0 0.0 0.0) Pawn (`self.AcceptanceRadius`)
      (:`OnSuccess`
        (`self.Attack`)))))

(event `Attack`
  (bind _mesh (`self.Mesh`))
  ;[1 0.7149 0 1 50] Pawn Sense + Attack
  (if (not (`/Game/ThirdPerson/Systems/DamageSystem/DamageSystem_BPC.bIsDead` (`self.DamageSystem_BPC`)))
    (`/Engine/EditorBlueprintResources/StandardMacros.DoOnce` false :!label _label
      (:`Completed`
        (bind _notifyname (`|PlayMontage` (`self.Mesh`) (`KismetArrayLibrary.Array_Random` (`|MakeArray` "/Game/Enemy/Robots/Robot1/Animations/TwoHanded_Attack3_Montage.TwoHanded_Attack3_Montage" "/Game/Enemy/Robots/Robot1/Animations/TwoHanded_Attack4_Montage.TwoHanded_Attack4_Montage" :!type "AnimMontage Object Reference")))
          (:`OnCompleted`
            (goto _label :!via `Reset`))
          (:`OnInterrupted`
            (`KismetSystemLibrary.Delay` 1.0)
            (goto _label :!via `Reset`))
          (:`OnNotifyBegin`
            (switch `name` _notifyname
              (:`Strike`
                (bind (_outhit _returnvalue) (`KismetSystemLibrary.SphereTraceSingleForObjects` (`SceneComponent.GetSocketLocation` _mesh "WeaponBase") (`SceneComponent.GetSocketLocation` _mesh "WeaponTip") 50.0 (`|MakeArray` "ObjectTypeQuery3" :!type "EObjectTypeQuery Enum")))
                (if _returnvalue
                  (bind (_bblockinghit _binitialoverlap _time _distance _location _impactpoint _normal _impactnormal _physmat _hitactor) (`GameplayStatics.BreakHitResult` _outhit))
                  (if (`self.ActorHasTag` _hitactor "Player")
                    (bind _wasdamaged (message `/Game/ThirdPerson/Systems/DamageSystem/Damageable_BPI.TakeDamage` _hitactor (make `/Game/ThirdPerson/Systems/DamageSystem/DamageInfo_S` 10.0 "NewEnumerator1" "NewEnumerator1")))
                    (if _wasdamaged
                      (`GameplayStatics.SpawnEmitterAtLocation` "/Game/StarterContent/Particles/P_Explosion.P_Explosion" _location))))))))))))

(event `YellowBlocked`
  (params (CanBeParried :type Boolean)))

(event `YellowDamageResponse`
  (params (DamageResponse :type "/Game/ThirdPerson/Systems/DamageSystem/DamageResponse_E Enum" :default "NewEnumerator0")))

(fn `GetCurrentHealth`
  (returns (Health :type "Float (double-precision)"))
  (return (`/Game/ThirdPerson/Systems/DamageSystem/DamageSystem_BPC.Health` (`self.DamageSystem_BPC`))))

(fn `GetMaxHealth`
  (returns (MaxHealth :type "Float (double-precision)"))
  (return (`/Game/ThirdPerson/Systems/DamageSystem/DamageSystem_BPC.MaxHealth` (`self.DamageSystem_BPC`))))

(fn `Heal`
  (params (Amount :type "Float (double-precision)"))
  (returns (NewHealth :type "Float (double-precision)"))
  (bind _newhealth (`/Game/ThirdPerson/Systems/DamageSystem/DamageSystem_BPC.Heal` (`self.DamageSystem_BPC`) Amount))
  (return _newhealth))

(fn `TakeDamage`
  (params (DamageInfo :type "/Game/ThirdPerson/Systems/DamageSystem/DamageInfo_S Structure"))
  (returns (WasDamaged :type Boolean))
  (bind _wasdamaged (`/Game/ThirdPerson/Systems/DamageSystem/DamageSystem_BPC.TakeDamage` (`self.DamageSystem_BPC`) DamageInfo))
  (return _wasdamaged))

(fn `UserConstructionScript`
  (bind _damagesystem_bpc (`self.DamageSystem_BPC`))
  (add `/Game/ThirdPerson/Systems/DamageSystem/DamageSystem_BPC.OnDeath` _damagesystem_bpc (`|CreateDelegate` :!event `YellowDeath`))
  (add `/Game/ThirdPerson/Systems/DamageSystem/DamageSystem_BPC.OnBlocked` _damagesystem_bpc (`|CreateDelegate` :!event `YellowBlocked`))
  (add `/Game/ThirdPerson/Systems/DamageSystem/DamageSystem_BPC.OnDamageResponse` _damagesystem_bpc (`|CreateDelegate` :!event `YellowDamageResponse`)))