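; Yellow arena end portal that appears once every yellow enemy in the level is dead.
; BeginPlay caches the player character and the initial list of BP_Enemy_Yellow actors.
; Each OpenEndPortalYellowArena call recounts enemies flagged YellowDead and compares that count to the initial list.
; On a match it unhides itself, spawns TeleporterYellow_BP at a hardcoded location after a short delay, and clears the player's current objective.
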(event `self.ReceiveBeginPlay`
  (bind _asbp_third_person_character (cast `/Game/ThirdPerson/Blueprints/BP_ThirdPersonCharacter` (`GameplayStatics.GetPlayerCharacter` 0)))
  (set `self.PlayerREF` _asbp_third_person_character)
  (bind _outactors (`GameplayStatics.GetAllActorsOfClass` "/Game/Enemy/BP_Enemy_Yellow.BP_Enemy_Yellow_C")))

(event `OpenEndPortalYellowArena`
  (`KismetArrayLibrary.Array_Clear` (`self.YellowEnemyREF`))
  (bind _outactors (`GameplayStatics.GetAllActorsOfClass` "/Game/Enemy/BP_Enemy_Yellow.BP_Enemy_Yellow_C"))
  (for _array_element _outactors
    (if (`/Game/Enemy/BP_Enemy_Yellow.YellowDead` _array_element)
      (`KismetArrayLibrary.Array_Add` (`self.YellowEnemyREF`) _array_element)))
  (if (== (`KismetArrayLibrary.Array_Length` (stale `self.ReceiveBeginPlay` _outactors)) (`KismetArrayLibrary.Array_Length` (`self.YellowEnemyREF`)))
    (`self.SetActorHiddenInGame` self false)
    (`KismetSystemLibrary.Delay` 0.2)
    (`|SpawnActorFromClass` "/Game/Blueprints/TeleporterYellow_BP.TeleporterYellow_BP_C" (`KismetMathLibrary.MakeTransform` (20215.0 -17731.0 2357.0)) "AlwaysSpawn" "MultiplyWithRoot" null null)
    (set `/Game/ThirdPerson/Blueprints/BP_ThirdPersonCharacter.CurrentObjective` "" (`self.PlayerREF`))))

(fn `UserConstructionScript`)