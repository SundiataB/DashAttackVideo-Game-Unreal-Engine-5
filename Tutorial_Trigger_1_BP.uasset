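; Tutorial trigger volume for the first step, teaching WASD movement and mouse controls.
; Shortly after BeginPlay, it disables jump and dash on any third-person character inside the box and spawns WASD and mouse text actors at fixed world locations.
; When the character leaves the box, jump is re-enabled while dash stays locked, and the box and both text actors are destroyed after a short delay.
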(event `self.ReceiveBeginPlay`
  (`KismetSystemLibrary.Delay` 0.2)
  (for _array_element (`PrimitiveComponent.GetOverlappingActors` (`self.Trigger1Box`) "/Game/ThirdPerson/Blueprints/BP_ThirdPersonCharacter.BP_ThirdPersonCharacter_C")
    (bind _asbp_third_person_character (cast `/Game/ThirdPerson/Blueprints/BP_ThirdPersonCharacter` _array_element))
    (set `/Game/ThirdPerson/Blueprints/BP_ThirdPersonCharacter.bCanJump` false _asbp_third_person_character)
    (set `/Game/ThirdPerson/Blueprints/BP_ThirdPersonCharacter.bCanDash` false _asbp_third_person_character)
    (bind _returnvalue (`|SpawnActorFromClass` "/Game/ThirdPerson/Systems/Tutorial/TutorialText/Trigs_Text/TutorialText_WASD_BP.TutorialText_WASD_BP_C" (`KismetMathLibrary.MakeTransform` (6440.0 0.0 500.0) (struct) (2.5 2.5 2.5)) "AlwaysSpawn" "MultiplyWithRoot" _asbp_third_person_character null))
    (set `self.WASDText_REF` _returnvalue)
    (bind _returnvalue_2 (`|SpawnActorFromClass` "/Game/ThirdPerson/Systems/Tutorial/TutorialText/Trigs_Text/TutorialText_Mouse_BP.TutorialText_Mouse_BP_C" (`KismetMathLibrary.MakeTransform` (6440.0 0.0 400.0) (struct) (2.5 2.5 2.5)) "AlwaysSpawn" "MultiplyWithRoot" null null))
    (set `self.MOUSEText_REF` _returnvalue_2)))

(event `self.Trigger1Box.OnComponentEndOverlap`
  (params (OverlappedComponent :type "PrimitiveComponent Object Reference") (OtherActor :type "Actor Object Reference") (OtherComp :type "PrimitiveComponent Object Reference") (OtherBodyIndex :type Integer))
  (`KismetSystemLibrary.Delay` 0.2)
  (bind _asbp_third_person_character (cast `/Game/ThirdPerson/Blueprints/BP_ThirdPersonCharacter` OtherActor))
  (set `/Game/ThirdPerson/Blueprints/BP_ThirdPersonCharacter.bCanJump` true _asbp_third_person_character)
  (set `/Game/ThirdPerson/Blueprints/BP_ThirdPersonCharacter.bCanDash` false _asbp_third_person_character)
  (`ActorComponent.K2_DestroyComponent` (`self.Trigger1Box`))
  (`self.K2_DestroyActor` (`self.WASDText_REF`))
  (`self.K2_DestroyActor` (`self.MOUSEText_REF`)))

(fn `UserConstructionScript`)