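; BP_TriggerPlasma is a trigger actor that shows a plasma ball's electricity effect while the player is inside its ActivatePlasma volume.
; On BeginPlay it caches the first BP_PlasmaBall found in the level, printing debug success or failure messages.
; Overlap begin and end events, filtered by the Player tag, unhide and hide that ball's Electricity component.
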(event `self.ReceiveBeginPlay`
  (bind _outactors (`GameplayStatics.GetAllActorsOfClass` "/Game/Blueprints/BP_PlasmaBall.BP_PlasmaBall_C"))
  (bind _asbp_plasma_ball (cast `/Game/Blueprints/BP_PlasmaBall` (`|GetArrayItem` _outactors))
    (:`then`
      (`KismetSystemLibrary.PrintString` "Cast Succed" true true (struct :`R` 0.098097 :`G` 1.0 :`A` 1.0) 10.0)
      (set `self.PlasmaBall_REF` _asbp_plasma_ball))
    (:`CastFailed`
      (`KismetSystemLibrary.PrintString` "Cast Failed" true true (struct :`R` 1.0 :`G` 0.081788 :`A` 1.0) 10.0))))

(event `self.Activate Plasma.OnComponentBeginOverlap`
  (params (OverlappedComponent :type "PrimitiveComponent Object Reference") (OtherActor :type "Actor Object Reference") (OtherComp :type "PrimitiveComponent Object Reference") (OtherBodyIndex :type Integer) (bFromSweep :type Boolean) (SweepResult :type "HitResult Structure (by ref)"))
  (if (`self.ActorHasTag` OtherActor "Player")
    (`SceneComponent.SetHiddenInGame` (`/Game/Blueprints/BP_PlasmaBall.Electricity` (`self.PlasmaBall_REF`)) false false)))

(event `self.Activate Plasma.OnComponentEndOverlap`
  (params (OverlappedComponent :type "PrimitiveComponent Object Reference") (OtherActor :type "Actor Object Reference") (OtherComp :type "PrimitiveComponent Object Reference") (OtherBodyIndex :type Integer))
  (if (`self.ActorHasTag` OtherActor "Player")
    (`SceneComponent.SetHiddenInGame` (`/Game/Blueprints/BP_PlasmaBall.Electricity` (`self.PlasmaBall_REF`)) true false)))

(fn `UserConstructionScript`)