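; Damage-causer Blueprint with a sphere overlap that hurts and knocks back yellow enemies while the player's dash type is Yellow.
; On overlap it checks the player's DashType gameplay tag and the other actor's Yellow and Enemy actor tags.
; A match stops the enemy's movement, sends it a fixed-damage TakeDamage message, then launches it along the forward vector of the player's FxLocation.
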(event `self.ReceiveBeginPlay`
  (bind _asbp_third_person_character (cast `/Game/ThirdPerson/Blueprints/BP_ThirdPersonCharacter` (`GameplayStatics.GetPlayerCharacter` 0)))
  (set `self.PlayerREF` _asbp_third_person_character))

(event `self.Sphere.OnComponentBeginOverlap`
  (params (OverlappedComponent :type "PrimitiveComponent Object Reference") (OtherActor :type "Actor Object Reference") (OtherComp :type "PrimitiveComponent Object Reference") (OtherBodyIndex :type Integer) (bFromSweep :type Boolean) (SweepResult :type "HitResult Structure (by ref)"))
  (if (and (`BlueprintGameplayTagLibrary.HasTag` (`/Game/ThirdPerson/Blueprints/BP_ThirdPersonCharacter.DashType` (`self.PlayerREF`)) (struct :`TagName` "State.Yellow") true) (`self.ActorHasTag` OtherActor "Yellow") (`self.ActorHasTag` OtherActor "Enemy"))
    (bind _asbp_enemy_yellow (cast `/Game/Enemy/BP_Enemy_Yellow` OtherActor))
    (bind _output_get (set `self.EnemyYellowREF` _asbp_enemy_yellow))
    (`MovementComponent.StopMovementImmediately` (`Character.CharacterMovement` _output_get))
    (bind _wasdamaged (message `/Game/ThirdPerson/Systems/DamageSystem/Damageable_BPI.TakeDamage` OtherActor (make `/Game/ThirdPerson/Systems/DamageSystem/DamageInfo_S` 25.0 "NewEnumerator1" "NewEnumerator1")))
    ;[1 0.7149 0 1 40] KNOCKBACK
    (`Character.LaunchCharacter` _output_get (* (`SceneComponent.GetForwardVector` (`/Game/ThirdPerson/Blueprints/BP_ThirdPersonCharacter.fx_location` (`self.PlayerREF`))) 4000.0) false false)
    (if _wasdamaged
      _)))

(fn `UserConstructionScript`)