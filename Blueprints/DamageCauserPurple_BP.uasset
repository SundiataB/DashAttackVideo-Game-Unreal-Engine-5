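; Damage-causer Blueprint that hurts purple enemies entering its sphere while the player's dash type is Purple.
; BeginPlay caches the third-person player character, whose DashType gameplay tags are checked for an exact State.Purple match on each sphere overlap.
; Overlapping actors tagged both Purple and Enemy are cast to BP_Enemy_Purple, have their movement stopped immediately, then receive fixed damage through a TakeDamage interface message.
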(event `self.ReceiveBeginPlay`
  ;[0.5 0 1 1 30] Begin Play + Overlap Sphere
  (bind _asbp_third_person_character (cast `/Game/ThirdPerson/Blueprints/BP_ThirdPersonCharacter` (`GameplayStatics.GetPlayerCharacter` 0)))
  (set `self.PlayerREF` _asbp_third_person_character))

(event `self.Sphere.OnComponentBeginOverlap`
  (params (OverlappedComponent :type "PrimitiveComponent Object Reference") (OtherActor :type "Actor Object Reference") (OtherComp :type "PrimitiveComponent Object Reference") (OtherBodyIndex :type Integer) (bFromSweep :type Boolean) (SweepResult :type "HitResult Structure (by ref)"))
  ;[0.5 0 1 1 30] Begin Play + Overlap Sphere
  (if (and (`BlueprintGameplayTagLibrary.HasTag` (`/Game/ThirdPerson/Blueprints/BP_ThirdPersonCharacter.DashType` (`self.PlayerREF`)) (struct :`TagName` "State.Purple") true) (`self.ActorHasTag` OtherActor "Purple") (`self.ActorHasTag` OtherActor "Enemy"))
    (bind _asbp_enemy_purple (cast `/Game/Enemy/BP_Enemy_Purple` OtherActor))
    (bind _output_get (set `self.EnemyPurpleREF` _asbp_enemy_purple))
    (`MovementComponent.StopMovementImmediately` (`Character.CharacterMovement` _output_get))
    (message `/Game/ThirdPerson/Systems/DamageSystem/Damageable_BPI.TakeDamage` OtherActor (make `/Game/ThirdPerson/Systems/DamageSystem/DamageInfo_S` 25.0 "NewEnumerator1" "NewEnumerator1"))))

(fn `UserConstructionScript`)