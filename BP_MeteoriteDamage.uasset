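; Boss missile strike marker that stages a delayed impact at its Plane's location, with no damage logic of its own.
; The scaleup event enlarges the actor, waits, then spawns a missile effect and BP_MissilesBoss.
; Two staggered explosions with sound follow, then it shakes the camera through the player reference cached at BeginPlay and destroys itself.
; A leftover scaling Timeline is never run.
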(event `self.ReceiveBeginPlay`
  ;[0.04239 1 0 0.5] Meg - Create Ref to player
  (bind _asbp_third_person_character (cast `/Game/ThirdPerson/Blueprints/BP_ThirdPersonCharacter` (`GameplayStatics.GetPlayerPawn` 0)))
  (set `self.PlayerRef` _asbp_third_person_character))

(event `scale up`
  (bind (_returnvalue_x _returnvalue_y) (`KismetMathLibrary.BreakVector` (`SceneComponent.K2_GetComponentLocation` (`self.Plane`))))
  (bind (_returnvalue_x_2 _returnvalue_y_2) (`KismetMathLibrary.BreakVector` (`SceneComponent.K2_GetComponentLocation` (`self.Plane`))))
  (bind _returnvalue (`SceneComponent.K2_GetComponentLocation` (`self.Plane`)))
  (`self.K2_SetActorTransform` (`KismetMathLibrary.MakeTransform` _returnvalue (struct) (10.0 10.0 1.0)))
  (`KismetSystemLibrary.Delay` 5.0)
  (`NiagaraFunctionLibrary.SpawnSystemAtLocation` "/Game/LevelPrototyping/Sundai/MissileForBoss/MissileForBoss.MissileForBoss" _returnvalue (struct :`Pitch` -90.0))
  (`|SpawnActorFromClass` "/Game/Blueprints/BP_MissilesBoss.BP_MissilesBoss_C" (`KismetMathLibrary.Conv_VectorToTransform` _returnvalue) "Undefined" "MultiplyWithRoot" null null)
  (`KismetSystemLibrary.Delay` 0.7)
  (`GameplayStatics.SpawnEmitterAtLocation` "/Game/StarterContent/Particles/P_Explosion.P_Explosion" (`KismetMathLibrary.MakeVector` (+ _returnvalue_x 5.0) (+ _returnvalue_y 5.0) 5.0) (struct) (10.0 10.0 10.0))
  (bind _output_get (set `self.Pitch Multiplier` (`KismetMathLibrary.FClamp` (`KismetMathLibrary.RandomFloat`) 0.5 1.5)))
  (`GameplayStatics.PlaySoundAtLocation` "/Game/StarterContent/Audio/Explosion01.Explosion01" (`SceneComponent.K2_GetComponentLocation` (`self.Plane`)) (struct) 0.7 _output_get 0.0 "/USDCore/USDDefaultAttenuation.USDDefaultAttenuation" null null null)
  (`KismetSystemLibrary.Delay` 0.3)
  (`GameplayStatics.SpawnEmitterAtLocation` "/Game/StarterContent/Particles/P_Explosion.P_Explosion" (`KismetMathLibrary.MakeVector` _returnvalue_x_2 _returnvalue_y_2 5.0) (struct) (15.0 15.0 15.0))
  (bind _output_get_2 (set `self.Pitch Multiplier` (`KismetMathLibrary.FClamp` (`KismetMathLibrary.RandomFloat`) 0.5 1.5)))
  (`GameplayStatics.PlaySoundAtLocation` "/Game/StarterContent/Audio/Explosion01.Explosion01" (`SceneComponent.K2_GetComponentLocation` (`self.Plane`)) (struct) 0.7 _output_get_2 0.0 "/USDCore/USDDefaultAttenuation.USDDefaultAttenuation" null null null)
  ;[0.04239 1 0 0.5] Meg - Add Camera Shake - (Camera shake component in Player BP)
  (`CameraShakeSourceComponent.StartCameraShake` :`self` (`/Game/ThirdPerson/Blueprints/BP_ThirdPersonCharacter.CameraShakeSource` (`self.PlayerRef`)) :`InCameraShake` "/Game/Enemy/Projectiles/BP_CameraShake.BP_CameraShake_C" :`Scale` 0.6)
  (`self.K2_DestroyActor`))

(fn `UserConstructionScript`)