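; BP_FloatingActors is a placeable prop that can be made to float when it is in an antigravity zone.
; Its construction script gives the static mesh a random mesh from an array and a random rotation for variety during placement.
; The ToggleGravity event switches the mesh's gravity on or off and applies a velocity-change impulse to propel it.
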(event `self.ReceiveBeginPlay`)

(event `/Game/Blueprints/BPI_AntiGravity.ToggleGravity`
  (params (hasGravity :type Boolean))
  (bind _staticmesh (`self.StaticMesh`))
  (`PrimitiveComponent.SetEnableGravity` _staticmesh hasGravity)
  ;[0.176 1 0 0.5] Meg - Creates slight impulse to propel mesh in antigravity zone
  (`PrimitiveComponent.AddImpulse` _staticmesh (`self.Impulse`) "None" true))

(fn `UserConstructionScript`
  ;[0 1 0.01766 0.5] Meg - preset static mesh while placing in world (random from an array)
  (`StaticMeshComponent.SetStaticMesh` (`self.StaticMesh`) (`KismetArrayLibrary.Array_Random` (`self.New Mesh`)))
  (`SceneComponent.K2_SetRelativeRotation` (`self.StaticMesh`) (`KismetMathLibrary.RandomRotator` true) false false))