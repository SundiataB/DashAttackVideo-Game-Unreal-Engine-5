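; A trigger volume that zooms the third-person camera in while the player stands inside it and back out on exit.
; BeginPlay caches the player's BP_ThirdPersonCharacter, then the Box overlap events check for the "Player" tag and play or reverse the POV timeline.
; The timeline lerps the CameraBoom arm length to a shorter distance; its socket offset lerp has identical endpoints, so that offset stays fixed.
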(event `self.ReceiveBeginPlay`
  (bind _asbp_third_person_character (cast `/Game/ThirdPerson/Blueprints/BP_ThirdPersonCharacter` (`GameplayStatics.GetPlayerCharacter` 0)))
  (set `self.PlayerREF` _asbp_third_person_character))

(event `self.Box.OnComponentBeginOverlap`
  (params (OverlappedComponent :type "PrimitiveComponent Object Reference") (OtherActor :type "Actor Object Reference") (OtherComp :type "PrimitiveComponent Object Reference") (OtherBodyIndex :type Integer) (bFromSweep :type Boolean) (SweepResult :type "HitResult Structure (by ref)"))
  (bind _cameraboom (`/Game/ThirdPerson/Blueprints/BP_ThirdPersonCharacter.CameraBoom` (`self.PlayerREF`)))
  (if (`self.ActorHasTag` OtherActor "Player")
    (bind (_direction _amount) (`Timeline|POV` :!label _label)
      (:`Update`
        (set `SpringArmComponent.TargetArmLength` (`KismetMathLibrary.Lerp` 300.0 200.0 _amount) _cameraboom)
        (set `SpringArmComponent.SocketOffset` (`KismetMathLibrary.VLerp` (0.0 0.0 25.0) (0.0 0.0 25.0) _amount) _cameraboom)))))

(event `self.Box.OnComponentEndOverlap`
  (params (OverlappedComponent :type "PrimitiveComponent Object Reference") (OtherActor :type "Actor Object Reference") (OtherComp :type "PrimitiveComponent Object Reference") (OtherBodyIndex :type Integer))
  (if (`self.ActorHasTag` OtherActor "Player")
    (goto _label :!via `Reverse`)))

(fn `UserConstructionScript`)